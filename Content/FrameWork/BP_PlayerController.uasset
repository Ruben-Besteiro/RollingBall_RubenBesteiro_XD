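; Player controller that owns the main HUD widget showing the player's lives and score.
; On BeginPlay it creates WBP_MainWidget, adds it to the viewport and seeds the lives text from CurrentLives.
; UpdateUILives and UpdateUIScore events pass new values to helper functions that write labelled text directly into the widget's text fields.
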(event EventBeginPlay
  ;[0.15 0.15 0.15 0.5] Inicializar UI
  (CallFunction|InitWidget)
  (CallFunction|SetLivesText (Variables|Default|GetCurrentLives)))

(event EventUpdateUILives
  (params (NewLives :type Integer))
  ;[0.15 0.15 0.15 0.5] Actualizar Nº de Vidas
  (CallFunction|SetLivesText NewLives))

(event EventUpdateUIScore
  (params (NewScore :type Integer))
  ;[0.15 0.15 0.15 0.5] Actualizar Score
  (CallFunction|SetScoreText NewScore))

(fn ConstructionScript)

(fn InitWidget
  (bind _returnvalue (UserInterface|CreateWidget "/Game/UI/WBP_MainWidget.WBP_MainWidget_C" self))
  (bind _output_get (Variables|Default|SetMyWidget _returnvalue))
  (UserInterface|Viewport|AddtoViewport _output_get 0))

(fn SetLivesText
  (params (NewLives :type Integer))
  (Rendering|Components|TextRender|SetText (Variables|/Game/UI/WBP_MainWidget.WBP_MainWidget_C|GetLivesText (Variables|Default|GetMyWidget)) (Utilities|Text|ToText(String) (Utilities|String|Append "Lives: " (Utilities|String|ToString(Integer) NewLives)))))

(fn SetScoreText
  (params (NewScore :type Integer))
  (Rendering|Components|TextRender|SetText (Variables|/Game/UI/WBP_MainWidget.WBP_MainWidget_C|GetScoreText (Variables|Default|GetMyWidget)) (Utilities|Text|ToText(String) (Utilities|String|Append "Score: " (Utilities|String|ToString(Integer) NewScore)))))